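; BP_OxygenProjectile is a projectile that, on hit, knocks back the player and nearby objects, then destroys itself after a short delay.
; A debug-drawn multi-sphere trace around the collider finds targets and applies linear-falloff radial impulses to non-player components.
; Player hits trigger LaunchCharacter away from the impact with added lift, using an unnormalized offset, so launch strength grows with distance.
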(event OnComponentHit(SphereCollider)
  (params (HitComponent :type Primitive%20Component%20Object%20Reference) (OtherActor :type Actor%20Object%20Reference) (OtherComp :type Primitive%20Component%20Object%20Reference) (NormalImpulse :type Vector :default "0, 0, 0") (Hit :type Hit%20Result%20Structure%20%28by%20ref%29))
  (bind _spherecollider (Variables|Default|GetSphereCollider))
  (bind _returnvalue (Transformation|GetWorldLocation _spherecollider))
  (Variables|Default|SetImpact%20Point (.ImpactPoint (Collision|BreakHitResult Hit)))
  (bind _outhits (Collision|MultiSphereTraceByChannel _returnvalue _returnvalue 2.5e+02 "TraceTypeQuery3" false 0 "ForDuration" true "(R=1.000000,G=0.000000,B=0.000000,A=1.000000)" "(R=0.000000,G=1.000000,B=0.000000,A=1.000000)" 2.5))
  (for _array_element _outhits
    (if (== (Components|GetOwner (.HitComponent (Collision|BreakHitResult _array_element))) (Game|GetPlayerCharacter 0))
      (bind _playerdirection (CallFunction|CalculatePlayerDistance (Variables|Default|GetImpact%20Point)))
      (Character|LaunchCharacter (Game|GetPlayerCharacter 0) (+ (* _playerdirection (Variables|Default|GetPlayerImpulseStrength)) "0.000000,0.000000,500.000000") false false)
      (Development|PrintString "Hello" true true "(R=0.000000,G=0.660000,B=1.000000,A=1.000000)" 1e+01 "8None")
      (else
        (Physics|AddRadialImpulse (.HitComponent (Collision|BreakHitResult _array_element)) (Transformation|GetWorldLocation (Variables|Default|GetSphereCollider)) 2.5e+02 (Variables|Default|GetImpulseStrength) "RIF_Linear" false) ; If not the player apply impulse
      )))
  (Utilities|FlowControl|Delay 0.2) ; Slight delay before removing projectile
  (Actor|DestroyActor))

(event EventBeginPlay)

(event Collision|EventActorBeginOverlap
  (params (OtherActor :type Actor%20Object%20Reference)))

(event EventTick
  (params (DeltaSeconds :type Float%20%28single-precision%29)))

(fn ConstructionScript)

(fn CalculatePlayerDistance
  (params (ImpactPoint :type Vector))
  (bind _returnvalue (Game|GetPlayerCharacter 0))
  (bind _capsulecomponent (Variables|/Script/Engine.Character|GetCapsuleComponent _returnvalue))
  (bind _returnvalue_2 (Transformation|GetWorldLocation _capsulecomponent))
  (return (- _returnvalue_2 ImpactPoint) (Math|Vector|Distance(Vector) _returnvalue_2 ImpactPoint)))