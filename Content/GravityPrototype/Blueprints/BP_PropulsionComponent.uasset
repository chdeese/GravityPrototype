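; Propulsion component that launches the player character opposite to the camera's look direction and can spawn oxygen projectiles along it.
; PropelPlayer scales the reversed camera forward vector by PropulsionStrength, then AngleCheck adds a stepped vertical boost for steep up or down aim, or a default lift.
; SpawnProjectile rotates a supplied scene component to the camera before spawning.
; Its own event graph drives nothing; the functions rely on external callers.
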(event EventBeginPlay)

(event EventTick
  (params (DeltaSeconds :type Float%20%28single-precision%29)))

(fn GetMouseClick
  (return (Math|Vector|GetForwardVector (Math|Rotator|FindLookatRotation (Transformation|GetWorldLocation (Variables|/Script/Engine.Character|GetCapsuleComponent (Game|GetPlayerCharacter 0))) (.TraceStart (Collision|BreakHitResult (.HitResult (Game|Player|GetHitResultUnderCursorbyChannel (Game|GetPlayerController 0) "TraceTypeQuery1" true))))))))

(fn SetPropulsionStrength
  (params (Input :type Float%20%28double-precision%29))
  (Variables|Default|SetPropulsionStrength Input))

(fn PropelPlayer
  ;[0.01764 0.01764 0.01764] GetVelocityFromCameraRotation
  (bind _rotation (CallFunction|GetCameraRotation))
  (bind _output_get (LocalVariables|SetVelocity (* _rotation (Variables|Default|GetPropulsionStrength))))
  (bind _returnvalue (CallFunction|AngleCheck (.z _output_get)))
  (Character|LaunchCharacter (Game|GetPlayerCharacter 0) (+ (LocalVariables|GetVelocity) (Math|Vector|MakeVector 0.0 0.0 _returnvalue)) false false))

(fn SpawnProjectile
  (params (ProjectileSpawnLocation :type Arrow%20Component%20Object%20Reference))
  (bind _output_get (Variables|Default|SetProjectile%20Spawn%20Location ProjectileSpawnLocation))
  (Transformation|SetWorldRotation _output_get (Transformation|GetWorldRotation (Actor|GetComponentbyClass (Game|GetPlayerCharacter 0) "/Script/Engine.CameraComponent")) false false) ; Stealing Camera's Rotation
  (Utilities|IsValid "/Game/GravityPrototype/Blueprints/BP_OxygenProjectile.BP_OxygenProjectile"
    (:Is%20Valid
      (Game|SpawnActorfromClass "/Game/GravityPrototype/Blueprints/BP_OxygenProjectile.BP_OxygenProjectile_C" (Transformation|GetWorldTransform (Variables|Default|GetProjectile%20Spawn%20Location)) "AlwaysSpawn" "MultiplyWithRoot" 0 0))))

(fn GetCameraRotation
  (return (* (Math|Vector|GetForwardVector (Transformation|GetWorldRotation (Actor|GetComponentbyClass (Game|GetPlayerCharacter 0) "/Script/Engine.CameraComponent"))) -1.0)))

(fn AngleCheck
  (params (A :type Float%20%28double-precision%29))
  (bind _output_get (LocalVariables|SetZaxis A))
  (if (< _output_get -6e+02)
    (bind _output_get_2 (LocalVariables|SetZaxis -1e+03)) ; Z Increase if aimed too high
    (return _output_get_2)
    (elif (> _output_get 9e+02)
      (bind _output_get_3 (LocalVariables|SetZaxis 1e+03)) ; Z Increse if aimed too low
      (return _output_get_3)
      (else
        (bind _output_get_4 (LocalVariables|SetZaxis 2e+02)) ; Default Z Increase
        (return _output_get_4)))))